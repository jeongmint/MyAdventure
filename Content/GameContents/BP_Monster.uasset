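; BP_Monster is an enemy actor that flies in a straight line, either toward the BP_SnowMan or straight down.
; On BeginPlay it finds the snowman and FindDirection picks a heading once: a 50% chance to aim at its current location, otherwise downward, which is also the fallback without a valid target.
; Tick moves the actor along that fixed direction by Speed and delta time, without sweep.
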(event EventBeginPlay
  (bind _returnvalue (Actor|GetActorOfClass "/Game/GameContents/BP_SnowMan.BP_SnowMan_C"))
  (Variables|Default|SetTarget _returnvalue)
  ;[1 1 1] 찾은 벡터 방향으로
  (CallFunction|FindDirection))

(event EventTick
  (params (DeltaSeconds :type Float%20%28single-precision%29))
  (Transformation|SetActorLocation (+ (Transformation|GetActorLocation) (* (* (Variables|Default|GetDirection) (Variables|Default|GetSpeed)) DeltaSeconds)) false false))

(fn ConstructionScript)

(fn FindDirection
  (bind _target (Variables|Default|GetTarget))
  (Utilities|IsValid _target
    (:Is%20Valid
      (if (<= (Math|Random|RandomIntegerinRange 1 100) 50)
        ;[1 1 1] True(50%초과 Player 추적)
        (Variables|Default|SetDirection (Math|Vector|Normalize (- (Transformation|GetActorLocation _target) (Transformation|GetActorLocation))))
        (else
          ;[1 1 1] False(50%이하 아래방향)
          (Variables|Default|SetDirection "0, 0,-1.000000" :!label _label))))
    (:Is%20Not%20Valid
      (goto _label))))